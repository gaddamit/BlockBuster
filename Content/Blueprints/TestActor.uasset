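; Actor for a 5x5 cube-grid puzzle where hits switch cells on or off to match a randomized target pattern, sliding into position after BeginPlay.
; Construction script indexes child cubes by name and randomizes starting and target states.
; OnCellCubeHit uses the UI's selected block shape and edge-checked index offsets to update cell state and material.
; Only the single-cell block checks for level clear; number keys set a local CurrentBlock or print debug text.
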(event Custom|StopMoving
  (Components|MoveComponentTo (Variables|Default|GetDefaultSceneRoot) (Variables|Default|GetTarget%20Location) "0, 0, 0" false false (Variables|Default|GetMoveSpeed) false) ; enters at Stop
)

(event EventBeginPlay
  (Utilities|FlowControl|Delay 0.2)
  (Components|MoveComponentTo (Variables|Default|GetDefaultSceneRoot) (Variables|Default|GetTarget%20Location) "0, 0, 0" false false (Variables|Default|GetMoveSpeed) false))

(event Input|KeyboardEvents|1
  (params (Key :type Key%20Structure :default "None"))
  (:Pressed
    (Development|PrintString "Hello")))

(event Input|KeyboardEvents|2
  (params (Key :type Key%20Structure :default "None"))
  (:Pressed
    (Variables|Default|SetCurrentBlock 2)))

(event Input|KeyboardEvents|3
  (params (Key :type Key%20Structure :default "None"))
  (:Pressed
    (Variables|Default|SetCurrentBlock 3)))

(event Input|KeyboardEvents|4
  (params (Key :type Key%20Structure :default "None"))
  (:Pressed
    (Variables|Default|SetCurrentBlock 4)))

(event Input|KeyboardEvents|5
  (params (Key :type Key%20Structure :default "None"))
  (:Pressed
    (Variables|Default|SetCurrentBlock 5)))

(event Input|KeyboardEvents|6
  (params (Key :type Key%20Structure :default "None"))
  (:Pressed
    (Variables|Default|SetCurrentBlock 6)))

(event Input|KeyboardEvents|7
  (params (Key :type Key%20Structure :default "None"))
  (:Pressed
    (Variables|Default|SetCurrentBlock 7)))

(event Input|KeyboardEvents|8
  (params (Key :type Key%20Structure :default "None"))
  (:Pressed
    (Variables|Default|SetCurrentBlock 8)))

(fn ConstructionScript
  (bind _returnvalue (Math|Random|RandomIntegerinRange 0 24))
  (for _array_element (Components|GetChildrenComponents (Variables|Default|GetDefaultSceneRoot) false)
    (if (Utilities|String|Contains (Utilities|GetObjectName _array_element) "Cube")
      (bind _asstatic_mesh_component (Utilities|Casting|CastToStaticMeshComponent _array_element))
      (Utilities|Array|SetArrayElem (Variables|Default|GetCubes) (- (Math|Conversions|ToInteger(Byte) (Utilities|String|GetSubstring (Utilities|GetObjectName _array_element) 4 2)) 1) _asstatic_mesh_component)))
  (while (!= (Variables|Default|GetConvertCubes) 0)
    (Utilities|Array|SetArrayElem (Variables|Default|GetCubeStatus) _returnvalue false)
    (CallFunction|SetCubeMaterialat _returnvalue false)
    (Math|Integer|DecrementInt (Variables|Default|GetConvertCubes)))
  (Variables|Default|SetConvertCubes (Variables|Default|GetDefaultConvertCubes))
  (while (!= (Variables|Default|GetConvertCubes) 0)
    (Utilities|Array|SetArrayElem (Variables|Default|GetTargetCubeStatus) (Math|Random|RandomIntegerinRange 0 24) false)
    (Math|Integer|DecrementInt (Variables|Default|GetConvertCubes))))

(fn OnCellCubeHit
  (params (Cube :type Static%20Mesh%20Component%20Object%20Reference) (IsUnion :type Boolean))
  (bind _ui (Variables|Default|GetUI))
  (bind _currentblock (Variables|/Game/Blueprints/SampleUI.SampleUI_C|GetCurrentBlock _ui))
  (LocalVariables|SetHitCube Cube)
  (for (_array_element _array_index) (Variables|Default|GetCubes)
    (if (== _array_element (LocalVariables|GetHitCube))
      (Variables|Default|SetBlockIndex _array_index)
      (Utilities|Array|Clear (Variables|Default|GetIndexToUpdate))
      (switch int _currentblock
        (:1
          (CallFunction|UpdateCube (Variables|Default|GetBlockIndex) IsUnion)
          (Variables|Default|SetIsLevelCleared true)
          (bind (_array_element_2 _array_index_2) (Utilities|Array|ForEachLoopwithBreak (Variables|Default|GetTargetCubeStatus) :!label _label)
            (:LoopBody
              (if (not (== _array_element_2 (Utilities|Array|Get(acopy) (Variables|Default|GetCubeStatus) _array_index_2)))
                (Development|PrintString (Utilities|String|ToString(Integer) _array_index_2))
                (Variables|Default|SetIsLevelCleared false)
                (goto _label Break)))
            (:Completed
              (if (Variables|Default|GetIsLevelCleared)
                (Development|PrintString "Level Cleared")))))
        (:2
          (CallFunction|GetIndiceswithType (Variables|Default|GetBlockIndex) _currentblock 0.0 :!label _label_2)
          (for _array_element_3 (Variables|Default|GetIndexToUpdate)
            (CallFunction|UpdateCube _array_element_3 IsUnion)))
        (:3
          (goto _label_2))
        (:4
          (goto _label_2))
        (:5
          (goto _label_2))
        (:6
          (goto _label_2))
        (:7
          (goto _label_2))
        (:8
          (goto _label_2))))))

(fn SetCubeMaterialat
  (params (Index :type Integer) (IsOn :type Boolean))
  (Rendering|Material|SetMaterial (Utilities|Array|Get(acopy) (Variables|Default|GetCubes) Index) 0 (select IsOn (Variables|Default|GetMaterialOn) (Variables|Default|GetMaterialOff))))

(fn UpdateCube
  (params (Index :type Integer) (IsUnion :type Boolean))
  (Utilities|Array|SetArrayElem (Variables|Default|GetCubeStatus) Index IsUnion)
  (CallFunction|SetCubeMaterialat Index IsUnion))

(fn GetIndiceswithType
  (params (BlockIndex :type Integer) (CurrentBlock :type Integer) (Rotation :type Float%20%28double-precision%29))
  (Utilities|Array|Add (Variables|Default|GetIndexToUpdate) BlockIndex)
  (switch int CurrentBlock
    (:2
      (|Block2))
    (:3
      (|Block3))
    (:4
      (Utilities|FlowControl|Sequence
        (:then_0
          (if (|({02E06CFC-224E-ECE8-A907-A4A12C355669}>4))
            (Utilities|Array|Add (Variables|Default|GetIndexToUpdate) (|({02E06CFC-224E-ECE8-A907-A4A12C355669}-5)))))
        (:then_1
          (if (|((((({02E06CFC-224E-ECE8-A907-A4A12C355669}!=4)&&({02E06CFC-224E-ECE8-A907-A4A12C355669}!=9))&&({02E06CFC-224E-ECE8-A907-A4A12C355669}!=14))&&({02E06CFC-224E-ECE8-A907-A4A12C355669}!=19))&&({02E06CFC-224E-ECE8-A907-A4A12C355669}!=24)))
            (Utilities|Array|Add (Variables|Default|GetIndexToUpdate) (|({02E06CFC-224E-ECE8-A907-A4A12C355669}+1)))))
        (:then_2
          (if (|({02E06CFC-224E-ECE8-A907-A4A12C355669}<19))
            (Utilities|Array|Add (Variables|Default|GetIndexToUpdate) (|({02E06CFC-224E-ECE8-A907-A4A12C355669}+6)))))))
    (:5
      (Utilities|FlowControl|Sequence
        (:then_0
          (if (|({02E06CFC-224E-ECE8-A907-A4A12C355669}>4))
            (Utilities|Array|Add (Variables|Default|GetIndexToUpdate) (|({02E06CFC-224E-ECE8-A907-A4A12C355669}-5)))))
        (:then_1
          (if (|((((({02E06CFC-224E-ECE8-A907-A4A12C355669}!=0)&&({02E06CFC-224E-ECE8-A907-A4A12C355669}!=5))&&({02E06CFC-224E-ECE8-A907-A4A12C355669}!=10))&&({02E06CFC-224E-ECE8-A907-A4A12C355669}!=15))&&({02E06CFC-224E-ECE8-A907-A4A12C355669}!=20)))
            (Utilities|Array|Add (Variables|Default|GetIndexToUpdate) (|({02E06CFC-224E-ECE8-A907-A4A12C355669}-1)))))
        (:then_2
          (if (|({02E06CFC-224E-ECE8-A907-A4A12C355669}<20))
            (Utilities|Array|Add (Variables|Default|GetIndexToUpdate) (|({02E06CFC-224E-ECE8-A907-A4A12C355669}+4)))))))
    (:6
      (|Block6))
    (:7
      (|Block7))
    (:8
      (|Block8))))