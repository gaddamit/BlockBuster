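; BP_Menu is a shootable level-select menu with Play, Tutorial and Endless components that react to hits from BP_Projectile.
; A hit swaps that component's material to EmissiveMeshMaterial, then to Glow after a short delay, and after a further pause opens the Game, Tutorial or Endless level.
; A shared IsTransitioning flag, set on the first hit and never cleared here, ignores any further selection during the transition.
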(event `self.Play.OnComponentHit`
  (params (HitComponent :type "PrimitiveComponent Object Reference") (OtherActor :type "Actor Object Reference") (OtherComp :type "PrimitiveComponent Object Reference") (NormalImpulse :type "Vector Structure") (Hit :type "HitResult Structure (by ref)"))
  (cast `/Game/Blueprints/BP_Projectile` OtherActor)
  (if (not (`self.IsTransitioning`))
    (set `self.IsTransitioning` true)
    (`PrimitiveComponent.SetMaterial` (`self.Play`) 0 "/Engine/EngineMaterials/EmissiveMeshMaterial.EmissiveMeshMaterial")
    (`KismetSystemLibrary.Delay` 0.25)
    (`PrimitiveComponent.SetMaterial` (`self.Play`) 0 "/Game/Materials/Glow.Glow")
    (`KismetSystemLibrary.Delay` 1.0)
    (`GameplayStatics.OpenLevel` "Game")))

(event `self.Tutorial.OnComponentHit`
  (params (HitComponent :type "PrimitiveComponent Object Reference") (OtherActor :type "Actor Object Reference") (OtherComp :type "PrimitiveComponent Object Reference") (NormalImpulse :type "Vector Structure") (Hit :type "HitResult Structure (by ref)"))
  (cast `/Game/Blueprints/BP_Projectile` OtherActor)
  (if (not (`self.IsTransitioning`))
    (set `self.IsTransitioning` true)
    (`PrimitiveComponent.SetMaterial` (`self.Tutorial`) 0 "/Engine/EngineMaterials/EmissiveMeshMaterial.EmissiveMeshMaterial")
    (`KismetSystemLibrary.Delay` 0.25)
    (`PrimitiveComponent.SetMaterial` (`self.Tutorial`) 0 "/Game/Materials/Glow.Glow")
    (`KismetSystemLibrary.Delay` 1.0)
    (`GameplayStatics.OpenLevel` "Tutorial")))

(event `self.Endless.OnComponentHit`
  (params (HitComponent :type "PrimitiveComponent Object Reference") (OtherActor :type "Actor Object Reference") (OtherComp :type "PrimitiveComponent Object Reference") (NormalImpulse :type "Vector Structure") (Hit :type "HitResult Structure (by ref)"))
  (cast `/Game/Blueprints/BP_Projectile` OtherActor)
  (if (not (`self.IsTransitioning`))
    (set `self.IsTransitioning` true)
    (`PrimitiveComponent.SetMaterial` (`self.Endless`) 0 "/Engine/EngineMaterials/EmissiveMeshMaterial.EmissiveMeshMaterial")
    (`KismetSystemLibrary.Delay` 0.25)
    (`PrimitiveComponent.SetMaterial` (`self.Endless`) 0 "/Game/Materials/Glow.Glow")
    (`KismetSystemLibrary.Delay` 1.0)
    (`GameplayStatics.OpenLevel` "Endless")))

(fn `UserConstructionScript`)