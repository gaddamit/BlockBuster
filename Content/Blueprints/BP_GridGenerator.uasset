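; Moving grid of 25 cubes in which two random cubes are marked as targets to hit, reporting cleared or not cleared.
; The grid moves to a target location, with rotation at level intervals, then destroys itself after a delay.
; Hit targets vanish; the last enables physics on every cube and stops movement.
; Tick triggers delayed cube swapping at level intervals, though both swap indices are 0, so positions stay unchanged.
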(event `self.ReceiveBeginPlay`
  (bind _rotator (`self.SetMovementRotation`))
  (`KismetSystemLibrary.MoveComponentTo` (`self.DefaultSceneRoot`) (`self.TargetLocation`) _rotator false false (+ (`self.BaseMovementTime`) (`KismetMathLibrary.RandomFloatInRange` (`self.MinAdjustMovementTIme`) (`self.MaxAdjustMovementTime`))) :!label _label)
  (`KismetSystemLibrary.Delay` (`self.DestroyDelay`))
  (`self.K2_DestroyActor`)
  (if (`self.IsCleared`)
    (`self.GridCleared`)
    (else
      (`self.GridNotCleared`))))

(event `StopMoving`
  (goto _label :!via `Stop`))

(event `self.ReceiveTick`
  (params (DeltaSeconds :type "Float (single-precision)"))
  (if (and (not (`self.IsCleared`)) (== (mod (`self.CurrentLevel`) (`self.SwapCubesAtLevelInterval`)) 0))
    (`KismetSystemLibrary.Delay` (`self.SwapCubesAtTimeInterval`))
    (`self.StartCubeSwapping`)))

(fn `GetRandomCube`
  (returns (Object :type "StaticMeshComponent Object Reference"))
  (bind _defaultsceneroot (`self.DefaultSceneRoot`))
  (bind _asstatic_mesh_component (cast `StaticMeshComponent` (`SceneComponent.GetChildComponent` _defaultsceneroot (`KismetMathLibrary.RandomInteger` (`SceneComponent.GetNumChildrenComponents` _defaultsceneroot)))))
  (return _asstatic_mesh_component))

(fn `OnCellCubeHit`
  (params (StaticMeshComponent :type "StaticMeshComponent Object Reference"))
  (returns (IsTarget :type Boolean))
  (locals (CurrentTarget :type "StaticMeshComponent Object Reference"))
  (bind _currenttarget (`local.CurrentTarget`))
  (set `local.CurrentTarget` StaticMeshComponent)
  (if (`KismetArrayLibrary.Array_Contains` (`self.TargetCubes`) (`local.CurrentTarget`))
    (bind _result (`/Engine/EditorBlueprintResources/StandardMacros.DecrementInt` (`self.TotalTargets`))
      (:`  `
        (if (== _result 0)
          (`PrimitiveComponent.SetSimulatePhysics` (`self.StaticMesh1`) true)
          (`PrimitiveComponent.SetSimulatePhysics` (`self.StaticMesh2`) true)
          (`PrimitiveComponent.SetSimulatePhysics` (`self.StaticMesh3`) true)
          (`PrimitiveComponent.SetSimulatePhysics` (`self.StaticMesh4`) true)
          (`PrimitiveComponent.SetSimulatePhysics` (`self.StaticMesh5`) true)
          (`PrimitiveComponent.SetSimulatePhysics` (`self.StaticMesh6`) true)
          (`PrimitiveComponent.SetSimulatePhysics` (`self.StaticMesh7`) true)
          (`PrimitiveComponent.SetSimulatePhysics` (`self.StaticMesh8`) true)
          (`PrimitiveComponent.SetSimulatePhysics` (`self.StaticMesh9`) true)
          (`PrimitiveComponent.SetSimulatePhysics` (`self.StaticMesh10`) true)
          (`PrimitiveComponent.SetSimulatePhysics` (`self.StaticMesh11`) true)
          (`PrimitiveComponent.SetSimulatePhysics` (`self.StaticMesh12`) true)
          (`PrimitiveComponent.SetSimulatePhysics` (`self.StaticMesh13`) true)
          (`PrimitiveComponent.SetSimulatePhysics` (`self.StaticMesh15`) true)
          (`PrimitiveComponent.SetSimulatePhysics` (`self.StaticMesh14`) true)
          (`PrimitiveComponent.SetSimulatePhysics` (`self.StaticMesh16`) true)
          (`PrimitiveComponent.SetSimulatePhysics` (`self.StaticMesh17`) true)
          (`PrimitiveComponent.SetSimulatePhysics` (`self.StaticMesh18`) true)
          (`PrimitiveComponent.SetSimulatePhysics` (`self.StaticMesh19`) true)
          (`PrimitiveComponent.SetSimulatePhysics` (`self.StaticMesh20`) true)
          (`PrimitiveComponent.SetSimulatePhysics` (`self.StaticMesh21`) true)
          (`PrimitiveComponent.SetSimulatePhysics` (`self.StaticMesh22`) true)
          (`PrimitiveComponent.SetSimulatePhysics` (`self.StaticMesh23`) true)
          (`PrimitiveComponent.SetSimulatePhysics` (`self.StaticMesh24`) true)
          (`PrimitiveComponent.SetSimulatePhysics` (`self.StaticMesh25`) true)
          (`self.StopMoving`)
          (set `self.IsCleared` true)
          (return true)
          (else
            (`PrimitiveComponent.SetCollisionEnabled` _currenttarget "NoCollision")
            (`SceneComponent.SetHiddenInGame` _currenttarget true false)
            (return true)))))))

(fn `SelectTargetCube`
  (returns (StaticMesh :type "StaticMeshComponent Object Reference"))
  (locals (TargetCube :type "StaticMeshComponent Object Reference"))
  (bind _targetcube (`local.TargetCube`))
  (bind _object (`self.GetRandomCube`))
  (set `local.TargetCube` _object)
  (while (`KismetArrayLibrary.Array_Contains` (`self.TargetCubes`) _targetcube)
    (bind _object_2 (`self.GetRandomCube`))
    (set `local.TargetCube` _object_2))
  (`PrimitiveComponent.SetMaterial` _targetcube 0 (`self.TargetMaterial`))
  (`KismetArrayLibrary.Array_Add` (`self.TargetCubes`) _targetcube)
  (return (`local.TargetCube`)))

(fn `SetLevel`
  (params (value :type Integer))
  (returns (CurrentGrid :type "/Game/Blueprints/BP_GridGenerator Object Reference"))
  (set `self.CurrentLevel` value)
  (return self))

(fn `SetMovementRotation`
  (returns (Rotator :type "Rotator Structure"))
  (locals (RotationSets :type "Array of Float (double-precision)"))
  (if (!= (mod (`self.CurrentLevel`) (`self.RotateGridAtLevelInterval`)) 0)
    (return)
    (else
      (return (`KismetMathLibrary.Conv_VectorToRotator` (`KismetMathLibrary.MakeVector` 0.0 0.0 (`KismetArrayLibrary.Array_Random` (`local.RotationSets`))))))))

(fn `StartCubeSwapping`
  (locals (CubeToSwap :type "StaticMeshComponent Object Reference"))
  (set `local.CubeToSwap` (`|GetArrayItem` (`self.TargetCubes`)))
  (while (`KismetArrayLibrary.Array_Contains` (`self.TargetCubes`) (stale _object))
    (bind _object (`self.GetRandomCube`))
    (set `local.CubeToSwap` _object))
  (`self.SwapCubePositions` 0))

(fn `SwapCubePositions`
  (params (CubeIndex1 :type Integer) (CubeIndex2 :type Integer))
  (locals (TempRelativeLocation :type "Vector Structure"))
  (bind _returnvalue (`SceneComponent.GetChildComponent` (`self.DefaultSceneRoot`) CubeIndex2))
  (bind _returnvalue_2 (`SceneComponent.GetChildComponent` (`self.DefaultSceneRoot`) CubeIndex1))
  (set `local.TempRelativeLocation` (`SceneComponent.RelativeLocation` _returnvalue_2))
  (`SceneComponent.K2_SetRelativeLocation` _returnvalue_2 (`SceneComponent.RelativeLocation` _returnvalue) false false)
  (`SceneComponent.K2_SetRelativeLocation` _returnvalue (`local.TempRelativeLocation`) false false))

(fn `UserConstructionScript`
  (`self.SelectTargetCube`)
  (`self.SelectTargetCube`))